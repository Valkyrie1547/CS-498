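; Spawner actor that builds a chain of BP_Tunnel segments, with random health packs and enemies.
; On BeginPlay it clears existing tunnels and health packs, then spawns an initial run starting at the player pawn.
; Each later segment attaches at the newest tunnel's SpawnPoint, and every segment gets a randomized wall and a reference back to the spawner.
; A random roll per segment may add a health pack, otherwise possibly an enemy, at a jittered offset.
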(event `self.ReceiveBeginPlay`
  (`self.SpawnInitialTunnels`))

(fn `Spawn Tunnel At Spawn Point`
  (locals (NewLocalVar_0 :type "Vector Structure" :default (0.0 0.0 0.0)))
  (`self.SpawnTunnel` (`SceneComponent.K2_GetComponentLocation` (`/Game/InfiniteMatrix/Blueprints/BP_Tunnel.SpawnPoint` (`self.NewestTunnel`)))))

(fn `SpawnEnemy`
  (params (SpawnLocation :type "Vector Structure"))
  (bind _returnvalue (`|SpawnActorFromClass` "/Game/InfiniteMatrix/Blueprints/Enemy.Enemy_C" (`KismetMathLibrary.MakeTransform` SpawnLocation (struct :`Yaw` 90.0)) "Undefined" "OverrideRootScale" null null))
  (set `self.NewestEnemy` _returnvalue))

(fn `SpawnHealthPack`
  (params (`Spawn Location` :type "Vector Structure"))
  (bind _returnvalue (`|SpawnActorFromClass` "/Game/InfiniteMatrix/Blueprints/Health_Pack.Health_Pack_C" (`KismetMathLibrary.MakeTransform` `Spawn Location` (struct :`Yaw` 90.0)) "Undefined" "OverrideRootScale" null null))
  (set `self.NewestHealthPack` _returnvalue))

(fn `SpawnInitialTunnels`
  (`|ExecutionSequence`
    (:`then_0`
      (bind _outactors (`GameplayStatics.GetAllActorsOfClass` "/Game/InfiniteMatrix/Blueprints/BP_Tunnel.BP_Tunnel_C"))
      (for _array_element _outactors
        (`self.K2_DestroyActor` _array_element)
        (bind _outactors_2 (`GameplayStatics.GetAllActorsOfClass` "/Game/InfiniteMatrix/Blueprints/Health_Pack.Health_Pack_C"))
        (`self.K2_DestroyActor` _outactors_2)))
    (:`then_1`
      (for _ (range 3)
        (`/Engine/EditorBlueprintResources/StandardMacros.IsValid` (`self.NewestTunnel`)
          (:`Is Valid`
            (`self.Spawn Tunnel At Spawn Point`))
          (:`Is Not Valid`
            (`self.SpawnTunnel` (`self.K2_GetActorLocation` (`GameplayStatics.GetPlayerPawn` 0)))))))))

(fn `SpawnTunnel`
  (params (SpawnLocation :type "Vector Structure"))
  (locals (NewLocalVar_1 :type "Vector Structure"))
  (bind _returnvalue (`KismetMathLibrary.RandomFloatInRange` -200.0 200.0))
  (bind _returnvalue_2 (`KismetMathLibrary.RandomFloatInRange` -200.0 200.0))
  (bind _returnvalue_3 (`|SpawnActorFromClass` "/Game/InfiniteMatrix/Blueprints/BP_Tunnel.BP_Tunnel_C" (`KismetMathLibrary.MakeTransform` SpawnLocation) "Undefined" "OverrideRootScale" null null))
  (bind _output_get (set `self.NewestTunnel` _returnvalue_3))
  (set `/Game/InfiniteMatrix/Blueprints/BP_Tunnel.TunnelSpawner` self _output_get)
  (`/Game/InfiniteMatrix/Blueprints/BP_Tunnel.RandomizeWall` _output_get)
  (if (== (`KismetMathLibrary.RandomIntegerInRange` 0 5) 1)
    (bind _output_get_2 (set `self.Spawn Location` SpawnLocation))
    (`self.SpawnHealthPack` (`KismetMathLibrary.MakeVector` (+ (.x _output_get_2) (`KismetMathLibrary.RandomFloatInRange` 500.0 2000.0)) (+ (.y _output_get_2) _returnvalue_2) (+ (.z _output_get_2) _returnvalue_2)))
    (elif (== (`KismetMathLibrary.RandomIntegerInRange` 0 5) 3)
      (bind _output_get_3 (set `self.Spawn Location` SpawnLocation))
      (`self.SpawnEnemy` (`KismetMathLibrary.MakeVector` (+ (.x _output_get_3) (`KismetMathLibrary.RandomFloatInRange` 500.0 2000.0)) (+ (.y _output_get_3) _returnvalue) (+ (.z _output_get_3) _returnvalue))))))

(fn `UserConstructionScript`)